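; Blueprint function library of small math and string-formatting helpers for dates and vectors.
; Date2FloatStr uses the integer multiply-add helper to pack date and time into base-100 numbers, joined as a decimal-style timestamp with milliseconds after the dot.
; The time and millisecond parts lack zero padding, so their width varies.
; Vector2Str and Vector2D2Str produce comma-separated components, and FMultAdd is the float multiply-add counterpart.
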(fn `Date2FloatStr`
  (params (Date :type "DateTime Structure"))
  (returns (`Return Value` :type String))
  (bind (_year _month _day _hour _minute _second _millisecond) (`KismetMathLibrary.BreakDateTime` Date))
  (return (`KismetStringLibrary.Concat_StrStr` (`KismetStringLibrary.Conv_IntToString` (`self.IMultAdd` (`self.IMultAdd` _year 100 _month) 100 _day)) (`KismetStringLibrary.Conv_IntToString` (`self.IMultAdd` (`self.IMultAdd` _hour 100 _minute) 100 _second)) "." (`KismetStringLibrary.Conv_IntToString` _millisecond))))

(fn `FMultAdd`
  (params (P1 :type "Float (double-precision)") (P1Mul :type "Float (double-precision)") (P2 :type "Float (double-precision)"))
  (returns (`Return Value` :type "Float (double-precision)"))
  (return (+ (* P1 P1Mul) P2)))

(fn `IMultAdd`
  (params (P1 :type Integer) (P1Mul :type Integer) (P2 :type Integer))
  (returns (`Return Value` :type Integer))
  (return (+ (* P1 P1Mul) P2)))

(fn `Vector2D2Str`
  (params (Vector :type "Vector2D Structure"))
  (returns (Str :type String))
  (bind (_x _y) (`KismetMathLibrary.BreakVector2D` Vector))
  (return (`KismetStringLibrary.JoinStringArray` (`|MakeArray` (`KismetStringLibrary.Conv_DoubleToString` _x) (`KismetStringLibrary.Conv_DoubleToString` _y)) ",")))

(fn `Vector2Str`
  (params (Vector :type "Vector Structure"))
  (returns (Str :type String))
  (return (`KismetStringLibrary.JoinStringArray` (`|MakeArray` (`KismetStringLibrary.Conv_DoubleToString` (.x Vector)) (`KismetStringLibrary.Conv_DoubleToString` (.y Vector)) (`KismetStringLibrary.Conv_DoubleToString` (.z Vector))) ",")))