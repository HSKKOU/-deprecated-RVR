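; MathLib is a Blueprint function library with integer and float multiply-add helpers and a date-to-numeric-string converter.
; Date2FloatStr nests IMultAdd to pack year-month-day and hour-minute-second into two base-100 integers, then joins them as text with a dot and milliseconds.
; The time and millisecond parts are not zero-padded, so the string length varies.
; FMultAdd is not used by the converter.
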(fn `Date2FloatStr`
  (params (Date :type "DateTime Structure"))
  (returns (`Return Value` :type String))
  (bind (_year _month _day _hour _minute _second _millisecond) (`KismetMathLibrary.BreakDateTime` Date))
  (return (`KismetStringLibrary.Concat_StrStr` (`KismetStringLibrary.Conv_IntToString` (`self.IMultAdd` (`self.IMultAdd` _year 100 _month) 100 _day)) (`KismetStringLibrary.Conv_IntToString` (`self.IMultAdd` (`self.IMultAdd` _hour 100 _minute) 100 _second)) "." (`KismetStringLibrary.Conv_IntToString` _millisecond))))

(fn `FMultAdd`
  (params (P1 :type "Float (double-precision)") (P1Mul :type "Float (double-precision)") (P2 :type "Float (double-precision)"))
  (returns (`Return Value` :type "Float (double-precision)"))
  (return (+ (* P1 P1Mul) P2)))

(fn `IMultAdd`
  (params (P1 :type Integer) (P1Mul :type Integer) (P2 :type Integer))
  (returns (`Return Value` :type Integer))
  (return (+ (* P1 P1Mul) P2)))