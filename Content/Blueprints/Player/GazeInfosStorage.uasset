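; GazeInfosStorage is an Actor Blueprint that buffers gaze info records, each carrying an ItemId.
; AddGazeInfo appends a record to GazeInfoArray and prints its ItemId, while Initialize resets the array.
; PopAllGazeInfoNow drains the buffer by copying it to a temporary array, clearing the original and returning the copy.
; The event graph and construction script are empty, so other code drives it through these functions.
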(fn `AddGazeInfo`
  (params (`New Info` :type "/Game/Blueprints/Player/GazeInfo Structure"))
  (`KismetArrayLibrary.Array_Add` (`self.GazeInfoArray`) `New Info`)
  (`KismetSystemLibrary.PrintString` (`KismetStringLibrary.Conv_IntToString` (`.itemId_12_6F18078F44F9685EF1C4BEAABE42DC56` (break `/Game/Blueprints/Player/GazeInfo` `New Info`))))
  (return))

(fn `Initialize`
  (set `self.GazeInfoArray` (`|MakeArray` (struct) :!type "/Game/Blueprints/Player/GazeInfo Structure"))
  (return))

(fn `PopAllGazeInfoNow`
  (returns (GazeInfoArrayPer :type "Array of /Game/Blueprints/Player/GazeInfo Structure"))
  (bind _gazeinfoarray (`self.GazeInfoArray`))
  (set `self.GazeInfoArrayTmp` _gazeinfoarray)
  (`KismetArrayLibrary.Array_Clear` _gazeinfoarray)
  (return (`self.GazeInfoArrayTmp`)))

(fn `UserConstructionScript`)