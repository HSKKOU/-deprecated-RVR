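; Player pawn with walk, sprint and yaw controls that records which items the player looks at and reports them to a server.
; Each Tick line-traces from the camera, with an input-adjustable end offset, for "Item"-tagged ItemActors.
; Hits are stored in a level-placed GazeInfosStorage actor with positions, gaze point and timestamp.
; A delayed loop from BeginPlay drains the storage, POSTs it as JSON and prints the response.
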(event Custom|OnComplete
  (params (Request :type Va%20Rest%20Request%20JSON%20Object%20Reference))
  ;[1 1 1] Post Gaze Info to Server
  (Connection|OnCompletePostInputs Request))

(event Custom|OnFailed
  (params (Request :type Va%20Rest%20Request%20JSON%20Object%20Reference))
  ;[1 1 1] Post Gaze Info to Server
  (Connection|OnFailedPostInputs Request))

(event EventBeginPlay
  (デフォルト|Initialize)
  ;[1 1 1] Loop with Delay
  (Utilities|FlowControl|Sequence :!label _label
    (:then_0
      (bind _gazeinfoarrayper (Default|PopAllGazeInfoNow (Variables|Default|GetGazeInfoStorage)))
      ;[1 1 1] Post Gaze Info to Server
      (bind (_newparam _success) (Connection|CreatePostInputsJson _gazeinfoarrayper))
      (if _success
        (bind _output_get (Variables|Default|SetRequest (Class|VaRestRequestJSON|ConstructRequestExt "POST" "json")))
        (Class|VaRestRequestJSON|SetRequestObject _output_get _newparam)
        (EventDispatchers|BindEventtoOnRequestComplete (Variables|Default|GetRequest) (delegate Custom|OnComplete))
        (EventDispatchers|BindEventtoOnRequestFail (Variables|Default|GetRequest) (delegate Custom|OnFailed))
        (Class|VaRestRequestJSON|ProcessURL (Variables|Default|GetRequest) (Variables|Default|GetPostUrl))))
    (:then_1
      (Utilities|FlowControl|Delay (Variables|Default|GetSendDelaySecond))
      (goto _label))))

(event Collision|EventActorBeginOverlap
  (params (OtherActor :type Actor%20Object%20Reference)))

(event EventTick
  (params (DeltaSeconds :type Float%20%28single-precision%29))
  ;[1 1 1] Tracing
  (bind (_iteminfo _itemlocation _gazeposition) (Controller|TraceGazeLine))
  (if (>= (.Id (Utilities|Struct|BreakItemInfo _iteminfo)) 0)
    (GazeStorage|AddGazeInfo (.Id (Utilities|Struct|BreakItemInfo _iteminfo)) _itemlocation _gazeposition)))

(event Input|ActionEvents|InputActionButtonX
  (params (Key :type Key%20Structure :default "AnyKey"))
  (bind _charactermovement (Variables|Character|GetCharacterMovement))
  ;[1 1 1] Movements
  (:Pressed
    (Variables|/Script/Engine.CharacterMovementComponent|SetMaxWalkSpeed _charactermovement (Variables|Movements|GetSprintSpeed)))
  (:Released
    (Variables|/Script/Engine.CharacterMovementComponent|SetMaxWalkSpeed _charactermovement (Variables|Movements|GetWalkSpeed))))

(event Input|AxisEvents|InputAxisMoveForward
  (params (AxisValue :type Float%20%28single-precision%29))
  ;[1 1 1] Movements
  (Pawn|Input|AddMovementInput (Math|Vector|GetForwardVector (Variables|/Script/Engine.PlayerCameraManager|GetTransformComponent (Game|GetPlayerCameraManager 0))) AxisValue false))

(event Input|AxisEvents|InputAxisGazeEndUp
  (params (AxisValue :type Float%20%28single-precision%29))
  ;[1 1 1] Fix Gaze End Point
  (Variables|GazeParanms|SetTraceEndPositionOffset (+ (Math|Vector|MakeVector 0.0 0.0 AxisValue) (Variables|GazeParanms|GetTraceEndPositionOffset))))

(event Input|AxisEvents|InputAxisMoveRight
  (params (AxisValue :type Float%20%28single-precision%29))
  ;[1 1 1] Movements
  (Pawn|Input|AddMovementInput (Math|Vector|GetRightVector (Variables|/Script/Engine.PlayerCameraManager|GetTransformComponent (Game|GetPlayerCameraManager 0))) AxisValue false))

(event Input|AxisEvents|InputAxisLookRight
  (params (AxisValue :type Float%20%28single-precision%29))
  ;[1 1 1] Movements
  (Pawn|Input|AddControllerYawInput (* AxisValue (Variables|Movements|GetLookRightReducer))))

(fn ConstructionScript)

(fn TraceGazeLine
  (bind _returnvalue (Game|GetPlayerCameraManager 0))
  (bind _returnvalue_2 (Transformation|GetActorLocation _returnvalue))
  (if (Variables|Default|GetIsInitialized)
    (bind (_outhit _returnvalue_3) (Collision|LineTraceByChannel _returnvalue_2 (+ (Variables|GazeParanms|GetTraceEndPositionOffset) _returnvalue_2 (* (Transformation|GetActorForwardVector _returnvalue) (Variables|GazeParanms|GetGazeTraceDist))) "TraceTypeQuery1" false 0 "ForOneFrame"))
    (if _returnvalue_3
      (if (Actor|ActorHasTag (.HitActor (Collision|BreakHitResult _outhit)) "Item")
        (if (.bSuccess (Utilities|Casting|CastToItemActor (.HitActor (Collision|BreakHitResult _outhit))))
          (bind _return_value (Default|GetItemInfo (.AsItem%20Actor (Utilities|Casting|CastToItemActor (.HitActor (Collision|BreakHitResult _outhit))))))
          (return _return_value (Transformation|GetActorLocation (.AsItem%20Actor (Utilities|Casting|CastToItemActor (.HitActor (Collision|BreakHitResult _outhit))))) (Default|CalcGazePoint (.AsItem%20Actor (Utilities|Casting|CastToItemActor (.HitActor (Collision|BreakHitResult _outhit)))) (.Location (Collision|BreakHitResult _outhit))))
          (else
            (return (Variables|Default|GetNullIntemInfo) "0, 0, 0" "")))
        (else
          (return (Variables|Default|GetNullIntemInfo) "0, 0, 0" "")))
      (else
        (return (Variables|Default|GetNullIntemInfo) "0, 0, 0" "")))
    (else
      (return (Variables|Default|GetNullIntemInfo) "0, 0, 0" ""))))

(fn AddGazeInfo
  (params (ItemId :type Integer) (ItemLocation :type Vector) (GazePosition :type Vector%202D%20Structure))
  (Default|AddGazeInfo (Variables|Default|GetGazeInfoStorage) (Utilities|Struct|MakeGazeInfo ItemId (Transformation|GetActorLocation) ItemLocation GazePosition (Utilities|Array|MakeArray 0) (Math|DateTime|Now))))

(fn InitializeGazeInfoStorage
  (bind _outactors (Actor|GetAllActorsOfClass "/Game/Blueprints/Player/GazeInfosStorage.GazeInfosStorage_C"))
  (bind _output_get (Variables|Default|SetGazeInfoStorage (Utilities|Array|Get(acopy) _outactors)))
  (Default|Initialize _output_get)
  (return))

(fn Initialize
  (GazeStorage|InitializeGazeInfoStorage)
  ;[1 1 1] Initialize Walk Speed
  (Variables|/Script/Engine.CharacterMovementComponent|SetMaxWalkSpeed (Variables|Character|GetCharacterMovement) (Variables|Movements|GetWalkSpeed))
  (Variables|Default|SetIsInitialized true)
  (return))

(fn CreatePostInputsJson
  (params (GazeInfoArray :type Array%20of%20Gaze%20Info%20Structures))
  (if (> (Utilities|Array|Length GazeInfoArray) 0)
    (for _array_element GazeInfoArray
      (bind _output_get (LocalVariables|SetJsonObjInFE (Class|VaRestJsonObject|ConstructJsonObject)))
      (Class|VaRestJsonObject|SetStringField _output_get "gaze_item_id" (Utilities|String|ToString(Integer) (.itemId (Utilities|Struct|BreakGazeInfo _array_element))))
      (Class|VaRestJsonObject|SetStringField _output_get "user_positionV3" (Utilities|String|ToString(Vector) (.userPosition (Utilities|Struct|BreakGazeInfo _array_element))))
      (Class|VaRestJsonObject|SetStringField _output_get "gaze_item_positionV3" (Utilities|String|ToString(Vector) (.itemPosition (Utilities|Struct|BreakGazeInfo _array_element))))
      (Class|VaRestJsonObject|SetStringField _output_get "gaze_pointV2" (Utilities|String|ToString(Vector2d) (.gazePosition (Utilities|Struct|BreakGazeInfo _array_element))))
      (Class|VaRestJsonObject|SetStringField _output_get "gaze_at_time" (CallFunction|Date2FloatStr (.gazeAtTime (Utilities|Struct|BreakGazeInfo _array_element))))
      (Utilities|Array|Add (LocalVariables|GetsendJsonObjArray) (LocalVariables|GetJsonObjInFE)))
    (LocalVariables|SetsendJsonObj (Class|VaRestJsonObject|ConstructJsonObject))
    (Class|VaRestJsonObject|SetObjectArrayField (LocalVariables|GetsendJsonObj) (LocalVariables|GetsendJsonObjField) (LocalVariables|GetsendJsonObjArray))
    (return (LocalVariables|GetsendJsonObj) true)
    (else
      (return (Class|VaRestJsonObject|ConstructJsonObject) false))))

(fn OnCompletePostInputs
  (params (Request :type Va%20Rest%20Request%20JSON%20Object%20Reference))
  (Development|PrintString (Variables|/Script/VaRestPlugin.VaRestRequestJSON|GetResponseContent Request)))

(fn OnFailedPostInputs
  (params (Request :type Va%20Rest%20Request%20JSON%20Object%20Reference))
  (Development|PrintString (Variables|/Script/VaRestPlugin.VaRestRequestJSON|GetResponseContent Request)))