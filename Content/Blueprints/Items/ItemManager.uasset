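; Item manager that fetches item data from a web API on BeginPlay and spawns an ItemActor for each entry.
; An HTTP GET response is parsed into ItemsInfo, then each actor receives its info and sprite URL.
; The active layout measures a throwaway actor but places every item at one point, InitialDist along X.
; An alternative layout distributing items across Tables exists but is disconnected in Initialize.
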(event Custom|OnComplete
  (params (Request :type Va%20Rest%20Request%20JSON%20Object%20Reference))
  (Server|OnCompleteGetItems Request))

(event Custom|OnFailed
  (params (Request :type Va%20Rest%20Request%20JSON%20Object%20Reference))
  (Development|PrintString "Failed"))

(event EventBeginPlay
  (Variables|Default|SetRequest (Class|VaRestRequestJSON|ConstructRequestExt "GET" "x_www_form_urlencoded_url"))
  (EventDispatchers|BindEventtoOnRequestComplete (Variables|Default|GetRequest) (delegate Custom|OnComplete))
  (EventDispatchers|BindEventtoOnRequestFail (Variables|Default|GetRequest) (delegate Custom|OnFailed))
  (Class|VaRestRequestJSON|ProcessURL (Variables|Default|GetRequest) (Variables|Default|GetUrlBase)))

(fn ConstructionScript)

(fn Initialize
  (Around|CreateItemsAroundUser) ; Around
  (return))

(fn CreateItem
  (params (ItemInfo :type Item%20Info%20Structure))
  (bind _returnvalue (Game|SpawnActorfromClass "/Game/Blueprints/Items/ItemActor.ItemActor_C" (Math|Transform|MakeTransform "0, 0, 0" "0, 0, 0" "1.000000,1.000000,1.000000") "Undefined" 0 0))
  (Default|InitializeStatus _returnvalue (Utilities|String|Append (LocalVariables|GetSpriteUrlBase) (.SpriteUrlStr (Utilities|Struct|BreakItemInfo ItemInfo))) ItemInfo)
  (Default|InitializeEvent _returnvalue)
  (return _returnvalue))

(fn CreateItemsEachTable
  (params (Table :type Table%20Actor%200%20Object%20Reference) (ItemInfoInTable :type Array%20of%20Item%20Info%20Structures))
  (Default|Initialize Table)
  (for _array_element ItemInfoInTable
    (bind _return_value (Item|CreateItem _array_element))
    (Utilities|Array|Add (LocalVariables|GetItemActors) _return_value))
  (Default|SetItems Table (LocalVariables|GetItemActors))
  (Default|LineUpItems Table))

(fn CreateItemsonTables
  (bind _itemsinfo (Variables|Default|GetItemsInfo))
  (LocalVariables|SetcurrentItemNum 0)
  (LocalVariables|SetnextItemNum -1)
  (for (_array_element _array_index) (Variables|Tables|GetTables)
    (Default|SetTableId _array_element _array_index)
    (CallFunction|AddEqInt (LocalVariables|GetnextItemNum) (Variables|/Game/Blueprints/Architectures/TableActor0.TableActor0_C|GetMaxItemNum _array_element))
    (Utilities|Array|Clear (LocalVariables|GetItemInfoInTable))
    (for _index (range (LocalVariables|GetcurrentItemNum) (LocalVariables|GetnextItemNum))
      (if (Utilities|Array|IsValidIndex (Variables|Default|GetItemsInfo) _index)
        (Utilities|Array|Add (LocalVariables|GetItemInfoInTable) (Utilities|Array|Get(acopy) (Variables|Default|GetItemsInfo) _index))
        (else
          (Utilities|Array|Add (LocalVariables|GetItemInfoInTable) (Utilities|Array|Get(acopy) _itemsinfo (Utilities|Array|LastIndex _itemsinfo))))))
    (Table|CreateItemsEachTable _array_element (LocalVariables|GetItemInfoInTable))
    (CallFunction|AddEqInt (LocalVariables|GetcurrentItemNum) (Variables|/Game/Blueprints/Architectures/TableActor0.TableActor0_C|GetMaxItemNum _array_element)))
  (return))

(fn OnCompleteGetItems
  (params (Response :type Va%20Rest%20Request%20JSON%20Object%20Reference))
  (bind _returnvalue (Class|VaRestRequestJSON|GetResponseObject Response))
  (if (Class|VaRestJsonObject|GetBoolField _returnvalue "result")
    (bind _returnvalue_2 (Class|VaRestJsonObject|GetObjectArrayField _returnvalue "data"))
    (for _array_element _returnvalue_2
      (Utilities|Array|Add (Variables|Default|GetItemsInfo) (Utilities|Struct|MakeItemInfo (Math|Float|Truncate (Class|VaRestJsonObject|GetNumberField _array_element "id")) (Class|VaRestJsonObject|GetStringField _array_element "name") (Math|Float|Truncate (Class|VaRestJsonObject|GetNumberField _array_element "prive")) (Class|VaRestJsonObject|GetStringField _array_element "description") (Class|VaRestJsonObject|GetStringField _array_element "url_image") 0 (Math|Float|Truncate (Class|VaRestJsonObject|GetNumberField _array_element "genre_id")))))
    (CallFunction|Initialize)
    (else
      (Development|PrintString "Failed Get Items Info"))))

(fn CreateItemsAroundUser
  (bind _returnvalue (Game|SpawnActorfromClass "/Game/Blueprints/Items/ItemActor.ItemActor_C" (Math|Transform|MakeTransform "0, 0, 0") "Undefined" 0 0))
  (LocalVariables|SetItemWidth (.X (Math|Vector|BreakVector (.BoxExtent (Collision|GetActorBounds _returnvalue false)))))
  (LocalVariables|SetItemHeight (.Z (Math|Vector|BreakVector (.BoxExtent (Collision|GetActorBounds _returnvalue false)))))
  (Actor|DestroyActor _returnvalue)
  (for _index (range 0 (Utilities|Array|LastIndex (Variables|Default|GetItemsInfo)))
    (bind _return_value (Item|CreateItem (Utilities|Array|Get(acopy) (Variables|Default|GetItemsInfo) _index)))
    (Transformation|SetActorLocation _return_value (Math|Vector|MakeVector (Variables|Around|GetInitialDist) 0.0 0.0) false false)))