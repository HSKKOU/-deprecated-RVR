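; ItemActor is a world actor that shows an item on a board using an image downloaded from a URL.
; InitializeStatus stores the transform, sprite URL and item info, then InitializeEvent downloads the image asynchronously.
; On success it writes the texture into the item info, applies it to the Board through a dynamic material instance, and moves the actor into place.
; Getter and setter functions expose the item info.
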(event `self.ReceiveBeginPlay`)

(event `InitializeEvent`
  (bind _texture (`AsyncTaskDownloadImage.DownloadImage` (`self.SpriteUrl`))
    (:`OnSuccess`
      (`self.InitializeItemInfo` _texture))))

(fn `GetItemInfo`
  (returns (`Return Value` :type "/Game/Blueprints/Items/ItemInfo Structure"))
  (return (`self.ItemInfo`)))

(fn `InitializeItemInfo`
  (params (texture :type "Texture2D Object Reference"))
  (bind (_id _name _price _description _sprite _review _genreid) (break `/Game/Blueprints/Items/ItemInfo` (`self.ItemInfo`)))
  (set `self.ItemInfo` (make `/Game/Blueprints/Items/ItemInfo` _id _name _price _description texture _review _genreid))
  (bind _returnvalue (`PrimitiveComponent.CreateDynamicMaterialInstance` (`self.Board`) 0 "/Game/Resources/Materials/ItemBaseMaterialInstance.ItemBaseMaterialInstance"))
  (`MaterialInstanceDynamic.SetTextureParameterValue` _returnvalue "BaseTexture" texture)
  (`self.InitializeTransform`)
  (return))

(fn `InitializeStatus`
  (params (Location :type "Vector Structure") (Rotation :type "Rotator Structure") (SpriteUrl :type String) (itemInfoWithoutSprite :type "/Game/Blueprints/Items/ItemInfo Structure"))
  (returns (`Return Value` :type Boolean))
  (set `self.Location` Location)
  (set `self.Rotation` Rotation)
  (set `self.SpriteUrl` SpriteUrl)
  (set `self.ItemInfo` itemInfoWithoutSprite)
  (return false))

(fn `InitializeTransform`
  (`self.K2_SetActorLocation` (`self.Location`))
  (`self.K2_SetActorRotation` (`self.Rotation`)))

(fn `SetItemInfo`
  (params (id :type Integer) (name :type String) (price :type Integer) (description :type String) (sprite :type "Texture2D Object Reference") (review :type "/Game/Blueprints/Items/ItemReviewInfo Structure") (genreId :type Integer))
  (set `self.ItemInfo` (make `/Game/Blueprints/Items/ItemInfo` id name price description sprite review genreId)))

(fn `UserConstructionScript`)