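; TableActor0 is a table actor that holds a set of item actors and lays them out in a row on its top.
; SetItems stores the items, and LineUpItems sums their widths to derive equal gaps across the table's Y bounds.
; It then places each item from the negative-Y edge, offset by its half height and half width.
; Initialize and the standard events are empty, and LineUpItems is not called within this Blueprint.
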(event EventBeginPlay)

(event Collision|EventActorBeginOverlap
  (params (OtherActor :type Actor%20Object%20Reference)))

(event EventTick
  (params (DeltaSeconds :type Float%20%28single-precision%29)))

(fn ConstructionScript)

(fn Initialize
  (return))

(fn SetItems
  (params (ItemInfos :type Array%20of%20Item%20Actor%20Object%20References))
  (Variables|Default|SetItemActors ItemInfos)
  (return))

(fn LineUpItems
  (bind (_origin _boxextent) (Collision|GetActorBounds false))
  (bind (_x _y _z) (Math|Vector|BreakVector _boxextent))
  (for _array_element (Variables|Default|GetItemActors)
    (LocalVariables|SetAllItemsWidth (+ (LocalVariables|GetAllItemsWidth) (.Y (Math|Vector|BreakVector (Default|GetActorWidthVector _array_element))))))
  (LocalVariables|SetEachMargin (Math|Vector|MakeVector 0.0 (/ (- (* 2 (.Y (Math|Vector|BreakVector (.BoxExtent (Collision|GetActorBounds false))))) (LocalVariables|GetAllItemsWidth)) (Math|Conversions|ToFloat(Integer) (+ (Utilities|Array|Length (Variables|Default|GetItemActors)) 1))) 0.0))
  (LocalVariables|SetLastPutItemLocation (+ _origin (Math|Vector|MakeVector 0.0 (* _y -1.0) _z) (LocalVariables|GetEachMargin)))
  (for _array_element_2 (Variables|Default|GetItemActors)
    (Transformation|SetActorLocationAndRotation _array_element_2 (+ (LocalVariables|GetLastPutItemLocation) (Default|GetActorHalfHeightVector _array_element_2) (Default|GetActorHalfWidthVector _array_element_2)))
    (LocalVariables|SetLastPutItemLocation (+ (LocalVariables|GetLastPutItemLocation) (LocalVariables|GetEachMargin) (Default|GetActorWidthVector _array_element_2)))))